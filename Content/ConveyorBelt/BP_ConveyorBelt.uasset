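; Conveyor belt actor that pushes actors overlapping its Box along the Arrow's forward vector each Tick, scaled by Speed.
; Movement pauses only while the Scan volume is overlapped and the belt is InUse.
; The Conveyor event toggles use mode, showing or removing W_ConveyorBelt, locking or restoring move input and the cursor, and setting InUse on every belt in the level.
; The Interact overlap handler is empty.
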(event OnComponentBeginOverlap(Scan)
  (params (OverlappedComponent :type Primitive%20Component%20Object%20Reference) (OtherActor :type Actor%20Object%20Reference) (OtherComp :type Primitive%20Component%20Object%20Reference) (OtherBodyIndex :type Integer) (bFromSweep :type Boolean) (SweepResult :type Hit%20Result%20Structure%20%28by%20ref%29))
  (Variables|Default|SetInScan true))

(event OnComponentEndOverlap(Scan)
  (params (OverlappedComponent :type Primitive%20Component%20Object%20Reference) (OtherActor :type Actor%20Object%20Reference) (OtherComp :type Primitive%20Component%20Object%20Reference) (OtherBodyIndex :type Integer))
  (Variables|Default|SetInScan false))

(event OnComponentBeginOverlap(Interact)
  (params (OverlappedComponent :type Primitive%20Component%20Object%20Reference) (OtherActor :type Actor%20Object%20Reference) (OtherComp :type Primitive%20Component%20Object%20Reference) (OtherBodyIndex :type Integer) (bFromSweep :type Boolean) (SweepResult :type Hit%20Result%20Structure%20%28by%20ref%29)))

(event EventBeginPlay)

(event Collision|EventActorBeginOverlap
  (params (OtherActor :type Actor%20Object%20Reference)))

(event EventTick
  (params (DeltaSeconds :type Float%20%28single-precision%29))
  (if (not (and (Variables|Default|GetInScan) (Variables|Default|GetInUse)))
    (for _array_element (Collision|GetOverlappingActors (Variables|Default|GetBox) 0 :!class /Script/Engine.PrimitiveComponent)
      (Transformation|AddActorWorldOffset _array_element (* (* DeltaSeconds (Variables|Default|GetSpeed)) (Math|Vector|GetForwardVector (Transformation|GetWorldRotation (Variables|Default|GetArrow))))))))

(event EventConveyor
  (if (Variables|Default|GetInUse)
    (CallFunction|StopConvey)
    (else
      (CallFunction|StartConvey))))

(fn ConstructionScript)

(fn StopConvey
  (bind _returnvalue (Game|GetPlayerController 0))
  (Widget|RemovefromParent (Variables|Default|GetUI))
  (Variables|Default|SetUI 0)
  (Input|ResetIgnoreMoveInput _returnvalue)
  (Variables|/Script/Engine.PlayerController|SetbShowMouseCursor _returnvalue false)
  (bind _outactors (Actor|GetAllActorsOfClass "BP_ConveyorBelt_C"))
  (for _array_element _outactors
    (bind _asbp_conveyor_belt (Utilities|Casting|CastToBP_ConveyorBelt _array_element))
    (Variables|BP_ConveyorBelt_C|SetInUse _asbp_conveyor_belt false)))

(fn StartConvey
  (bind _returnvalue (Game|GetPlayerController 0))
  (Input|SetIgnoreMoveInput _returnvalue true)
  (bind _returnvalue_2 (UserInterface|CreateWidget "/Game/ConveyorBelt/W_ConveyorBelt.W_ConveyorBelt_C" _returnvalue))
  (bind _output_get (Variables|Default|SetUI _returnvalue_2))
  (UserInterface|Viewport|AddtoViewport _output_get 0)
  (Variables|/Script/Engine.PlayerController|SetbShowMouseCursor (Game|GetPlayerController 0) true)
  (bind _outactors (Actor|GetAllActorsOfClass "BP_ConveyorBelt_C"))
  (for _array_element _outactors
    (bind _asbp_conveyor_belt (Utilities|Casting|CastToBP_ConveyorBelt _array_element))
    (Variables|BP_ConveyorBelt_C|SetInUse _asbp_conveyor_belt true)))